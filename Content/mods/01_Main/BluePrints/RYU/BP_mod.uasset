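; RYU mod skeletal mesh Blueprint that swaps in the mesh, physics asset and animation class from ModSettings at BeginPlay.
; SetMat then rebuilds each material slot holding a material instance constant as a dynamic instance of the MatTemp template.
; SetModMID copies listed texture and scalar parameters from the original material onto each new instance, carrying the mod's look over to the template.
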(event `self.ReceiveBeginPlay`
  (bind (_skinname _mesh _pa _abp) (break `/Game/mods/01_Main/BluePrints/Struct/S_SkinInfo` (`/Game/mods/01_Main/BluePrints/BP_PDA_settings.RYU` (`self.Mod Settings`))))
  (`self.SetSkeletalMeshAsset` _mesh)
  (`self.SetPhysicsAsset` _pa)
  (`self.SetAnimInstanceClass` _abp)
  (`self.Set Mat`))

(fn `Set Mat`
  (for _index (range (`self.GetNumMaterials`))
    (bind `_as材质实例常量` (cast `MaterialInstanceConstant` (`self.GetMaterial` _index)))
    (bind _returnvalue (`KismetMaterialLibrary.CreateDynamicMaterialInstance` (`self.MatTemp`)))
    (`self.SetMaterial` _index (`self.Set Mod MID` _returnvalue `_as材质实例常量`))))

(fn `Set Mod MID`
  (params (ModMID :type "MaterialInstanceDynamic Object Reference") (OldMat :type "MaterialInstanceConstant Object Reference"))
  (returns (ModifiedMID :type "MaterialInstanceDynamic Object Reference"))
  (locals (OM :type "MaterialInstanceConstant Object Reference") (MM :type "MaterialInstanceDynamic Object Reference"))
  (bind _om (`local.OM`))
  (bind _mm (`local.MM`))
  (set `local.OM` OldMat)
  (set `local.MM` ModMID)
  (`|ExecutionSequence`
    (:`then_0`
      (for _array_element (`self.Array_TextureParamNames`)
        (bind _returnvalue (`MaterialInstanceConstant.K2_GetTextureParameterValue` _om _array_element))
        (`MaterialInstanceDynamic.SetTextureParameterValue` _mm _array_element _returnvalue)))
    (:`then_1`
      (for _array_element_2 (`self.Array_ScaleParamNames`)
        (bind _returnvalue_2 (`MaterialInstanceConstant.K2_GetScalarParameterValue` _om _array_element_2))
        (`MaterialInstanceDynamic.SetScalarParameterValue` _mm _array_element_2 _returnvalue_2)))
    (:`then_2`
      (return (`local.MM`)))))