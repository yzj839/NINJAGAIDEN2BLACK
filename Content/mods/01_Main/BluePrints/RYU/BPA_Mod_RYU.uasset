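; BPA_Mod_RYU is a mod actor that manages the RYU skin and its own visibility.
; SetRYUSkin writes the skin info to ModSetting.RYU, then replaces any existing BPMod component with a new BP_mod.
; Each Tick it mirrors its attach parent's hidden state; unattached, it shows only while AA is valid.
; Logic for attaching to character or cutscene skeletal meshes remains in the graph, unconnected.
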(event `self.ReceiveTick`
  (params (DeltaSeconds :type "Float (single-precision)"))
  (bind _returnvalue (`self.GetAttachParentActor` self))
  (if (`KismetSystemLibrary.IsValid` _returnvalue)
    (`self.SetActorHiddenInGame` self (`Actor.bHidden` _returnvalue))
    (else
      (`self.AA`
        (:`then`
          (`self.SetActorHiddenInGame` false))
        (:`else`
          (`self.SetActorHiddenInGame` true))))))

(event `self.ReceiveBeginPlay`)

(event `/Game/mods/01_Main/BluePrints/IF_mod.Set RYU Skin`
  (params (SkinInfo :type "/Game/mods/01_Main/BluePrints/Struct/S_SkinInfo Structure"))
  ;[1 1 1] 注释
  (`|VariableSetRef` (`/Game/mods/01_Main/BluePrints/Struct/BP_PDA.RYU` (`self.ModSetting`)) SkinInfo)
  (bind _bp_mod (`self.BP_mod`)
    (:`then`
      (`ActorComponent.K2_DestroyComponent` _bp_mod))
    (:`else`
      _))
  (bind _returnvalue (`|AddComponentByClass` "/Game/mods/01_Main/BluePrints/RYU/BP_mod.BP_mod_C"))
  (set `self.BP_mod` _returnvalue))

(event `self.ReceiveDestroyed`)

(fn `UserConstructionScript`)